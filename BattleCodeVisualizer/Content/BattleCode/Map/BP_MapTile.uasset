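; BP_MapTile is a battle map tile actor with a Plane and an Obstacle mesh.
; The construction script gives each mesh its own dynamic instance of MI_Unit, tinting the plane green and the obstacle dark grey through the Color parameter.
; The SetStatus event stores the tile status and shows the obstacle only when that status equals 1, hiding it otherwise.
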(event Custom|SetStatus
  (params (Status :type Integer))
  (Variables|Default|SetStatus Status)
  (Development|SetHiddeninGame (Variables|Default|GetObstacle) (!= (Variables|Default|GetStatus) 1) false))

(fn ConstructionScript
  (bind _returnvalue (Rendering|Material|CreateDynamicMaterialInstance (Variables|Default|GetPlane) 0 "/Game/BattleCode/MI_Unit.MI_Unit" :!class /Script/Engine.PrimitiveComponent))
  (Rendering|Material|SetVectorParameterValue _returnvalue "Color" "(R=0.320344,G=1.000000,B=0.189238,A=1.000000)" :!class /Script/Engine.MaterialInstanceDynamic)
  (bind _returnvalue_2 (Rendering|Material|CreateDynamicMaterialInstance (Variables|Default|GetObstacle) 0 "/Game/BattleCode/MI_Unit.MI_Unit" :!class /Script/Engine.PrimitiveComponent))
  (Rendering|Material|SetVectorParameterValue _returnvalue_2 "Color" "(R=0.213542,G=0.201048,B=0.194536,A=1.000000)" :!class /Script/Engine.MaterialInstanceDynamic))