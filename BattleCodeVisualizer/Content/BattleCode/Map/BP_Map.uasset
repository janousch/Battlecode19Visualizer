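; Map actor that builds the battle grid at BeginPlay from the columns and rows in its BCMap data.
; It adds a BP_MapTile child actor at evenly spaced positions for each cell and passes the cell's value to SetStatus.
; Custom events drive the nested loop in place of loop nodes, with a brief Delay every few rows to spread spawning over time.
; When finished it prints the column count as a debug message.
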(event Custom|NextRow
  (bind _rowstocreate (Variables|Default|GetRowsToCreate))
  (if (Utilities|Array|IsValidIndex _rowstocreate (Variables|Default|GetCurrentRow))
    (bind _returnvalue (AddComponent|AddChildActorComponent false (Math|Transform|MakeTransform (Math|Vector|MakeVector (* (Variables|Default|GetCurrentRow) 4e+02) (* (Variables|Default|GetCurrentColumn) 4e+02) 0.0) "0, 0, 0" "1,1,1")))
    (bind _asbp_map_tile (Utilities|Casting|CastToBP_MapTile (Variables|/Script/Engine.ChildActorComponent|GetChildActor _returnvalue)))
    (Default|SetStatus _asbp_map_tile (Utilities|Array|Get(acopy) _rowstocreate (Variables|Default|GetCurrentRow)))
    (bind _result (Math|Integer|IncrementInt (Variables|Default|GetCurrentRow))
      (:%20%20
        (if (== (Math|Integer|%(Integer) _result 5) 0)
          (Utilities|FlowControl|Delay 0.01))
        (CallFunction|NextRow)))
    (else
      (Math|Integer|IncrementInt (Variables|Default|GetCurrentColumn)
        (:%20%20
          (Variables|Default|SetCurrentRow 0)
          (CallFunction|NextColumn))))))

(event Custom|NextColumn
  (bind _currentcolumn (Variables|Default|GetCurrentColumn))
  (bind _columnstocreate (Variables|Default|GetColumnsToCreate))
  (if (Utilities|Array|IsValidIndex _columnstocreate _currentcolumn)
    (Variables|Default|SetRowsToCreate (.rows (Utilities|Array|Get(acopy) _columnstocreate _currentcolumn)))
    (if (Utilities|Array|IsValidIndex (Variables|Default|GetRowsToCreate) (Variables|Default|GetCurrentRow))
      (bind _returnvalue (AddComponent|AddChildActorComponent false (Math|Transform|MakeTransform (Math|Vector|MakeVector (* (Variables|Default|GetCurrentRow) 4e+02) (* (Variables|Default|GetCurrentColumn) 4e+02) 0.0) "0, 0, 0" "1,1,1")))
      (bind _asbp_map_tile (Utilities|Casting|CastToBP_MapTile (Variables|/Script/Engine.ChildActorComponent|GetChildActor _returnvalue)))
      (Default|SetStatus _asbp_map_tile (Utilities|Array|Get(acopy) (Variables|Default|GetRowsToCreate) (Variables|Default|GetCurrentRow)))
      (bind _result (Math|Integer|IncrementInt (Variables|Default|GetCurrentRow))
        (:%20%20
          (if (== (Math|Integer|%(Integer) _result 5) 0)
            (Utilities|FlowControl|Delay 0.01))
          (CallFunction|NextRow)))
      (else
        (Math|Integer|IncrementInt (Variables|Default|GetCurrentColumn)
          (:%20%20
            (Variables|Default|SetCurrentRow 0)
            (CallFunction|NextColumn)))))
    (else
      (Development|PrintString (Utilities|String|Append "Width x Height = " (Utilities|String|ToString(Integer) (Utilities|Array|Length (Variables|Default|GetColumnsToCreate))))))))

(event EventBeginPlay
  (Variables|Default|SetColumnsToCreate (.columns (Variables|Default|GetBCMap)))
  (Variables|Default|SetCurrentColumn 0)
  (Variables|Default|SetCurrentRow 0)
  (if (Utilities|Array|IsValidIndex (Variables|Default|GetColumnsToCreate) (Variables|Default|GetCurrentColumn))
    (Variables|Default|SetRowsToCreate (.rows (Utilities|Array|Get(acopy) (Variables|Default|GetColumnsToCreate) (Variables|Default|GetCurrentColumn))))
    (if (Utilities|Array|IsValidIndex (Variables|Default|GetRowsToCreate) (Variables|Default|GetCurrentRow))
      (bind _returnvalue (AddComponent|AddChildActorComponent false (Math|Transform|MakeTransform (Math|Vector|MakeVector (* (Variables|Default|GetCurrentRow) 4e+02) (* (Variables|Default|GetCurrentColumn) 4e+02) 0.0) "0, 0, 0" "1,1,1")))
      (bind _asbp_map_tile (Utilities|Casting|CastToBP_MapTile (Variables|/Script/Engine.ChildActorComponent|GetChildActor _returnvalue)))
      (Default|SetStatus _asbp_map_tile (Utilities|Array|Get(acopy) (Variables|Default|GetRowsToCreate) (Variables|Default|GetCurrentRow)))
      (bind _result (Math|Integer|IncrementInt (Variables|Default|GetCurrentRow))
        (:%20%20
          (if (== (Math|Integer|%(Integer) _result 5) 0)
            (Utilities|FlowControl|Delay 0.01))
          (CallFunction|NextRow)))
      (else
        (Math|Integer|IncrementInt (Variables|Default|GetCurrentColumn)
          (:%20%20
            (Variables|Default|SetCurrentRow 0)
            (CallFunction|NextColumn)))))
    (else
      (Development|PrintString (Utilities|String|Append "Width x Height = " (Utilities|String|ToString(Integer) (Utilities|Array|Length (Variables|Default|GetColumnsToCreate))))))))

(fn ConstructionScript)