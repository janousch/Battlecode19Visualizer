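; BP_GameState is the game state for a BattleCode match, managing map creation and choosing a winning team.
; InitializeMap destroys a valid existing map, then spawns and stores a BP_Map built from the supplied map data.
; DetermineWinner compares red and blue castle counts, with ties sharing the not-more-red result; GetUnitValue is a stub returning zero.
; InitializeMapDep, apparently deprecated, spawns individual BP_MapTile actors on a grid.
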(event Custom|InitializeMap
  (params (Map :type BC%20Map%20Structure))
  (Utilities|IsValid (Variables|Default|GetMap)
    (:Is%20Valid
      (Actor|DestroyActor (Variables|Default|GetMap)))
    (:Is%20Not%20Valid
      _))
  (bind _returnvalue (Game|SpawnActorfromClass "/Game/BattleCode/Map/BP_Map.BP_Map_C" (Math|Transform|MakeTransform "0, 0, 0" "0, 0, 0" "1,1,1") "Undefined" 0 Map 0))
  (Variables|Default|SetMap _returnvalue))

(fn ConstructionScript)

(fn DetermineWinner
  (if (> (Utilities|Array|Length (Variables|Team|Red|GetCastlesRed)) (Utilities|Array|Length (Variables|Team|Blue|GetCastlesBlue)))
    (return "NewEnumerator1")
    (else
      (return "NewEnumerator0"))))

(fn GetUnitValue
  (params (Team :type ETeam%20Enum :default "NewEnumerator0"))
  (return 0))

(fn InitializeMapDep
  (params (Map :type BC%20Map%20Structure))
  (for (_array_element _array_index) (.columns Map)
    (for (_array_element_2 _array_index_2) (.rows _array_element)
      (Game|SpawnActorfromClass "/Game/BattleCode/Map/BP_MapTile.BP_MapTile_C" (Math|Transform|MakeTransform (Math|Vector|MakeVector (* _array_index (LocalVariables|GetOFFSET)) (* _array_index_2 (LocalVariables|GetOFFSET)) 0.0) "0, 0, 0" "1,1,1") "Undefined" 0 _array_element_2 0))))